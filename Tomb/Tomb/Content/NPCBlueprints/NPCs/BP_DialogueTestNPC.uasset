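; BP_DialogueTestNPC is a test NPC that opens a conversation when a player interacts with it.
; OnInteract stores the player, sends it EnterDialogueMessage with itself, then opens the conversation on its dialogue component.
; An interaction radius toggles a name label, set from CharacterName at construction, as the player character enters and leaves.
; Both the Interactable? and IsNPC? functions return false.
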(event `/Game/FirstPerson/Blueprints/Interfaces/BPI_Interactable.OnInteract`
  (params (InteractingPlayer :type "Character Object Reference"))
  (bind _output_get (set `self.InteractingPlayer` InteractingPlayer))
  (message `/Game/FirstPerson/Blueprints/Interfaces/BPI_Player.EnterDialogue` _output_get self)
  (`/Game/NPCBlueprints/DialogueComponent_Base.OpenConversation` (`self.DialogueComponent_TestNPC`)))

(event `self.InteractableRadius.OnComponentBeginOverlap`
  (params (OverlappedComponent :type "PrimitiveComponent Object Reference") (OtherActor :type "Actor Object Reference") (OtherComp :type "PrimitiveComponent Object Reference") (OtherBodyIndex :type Integer) (bFromSweep :type Boolean) (SweepResult :type "HitResult Structure (by ref)"))
  (if (== OtherActor (`GameplayStatics.GetPlayerCharacter` 0))
    (`SceneComponent.SetVisibility` (`self.Txt_CharacterName`) true false)))

(event `self.InteractableRadius.OnComponentEndOverlap`
  (params (OverlappedComponent :type "PrimitiveComponent Object Reference") (OtherActor :type "Actor Object Reference") (OtherComp :type "PrimitiveComponent Object Reference") (OtherBodyIndex :type Integer))
  (if (== OtherActor (`GameplayStatics.GetPlayerCharacter` 0))
    (`SceneComponent.SetVisibility` (`self.Txt_CharacterName`) false false)))

(fn `Interactable?`
  (returns (`Interactable?` :type Boolean))
  (return false))

(fn `IsNPC?`
  (returns (`IsNPC?` :type Boolean))
  (return false))

(fn `UserConstructionScript`
  (`TextRenderComponent.K2_SetText` (`self.Txt_CharacterName`) (`self.CharacterName`)))