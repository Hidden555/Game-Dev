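; AI controller for the SKnight enemy that runs its behavior tree on BeginPlay and feeds it what the enemy sees.
; Perception updates are filtered to sight stimuli from the player character.
; A sighting sets the TargetActor blackboard key to the player.
; Losing sight clears that key and stores the stimulus location as LastKnownLocation.
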(event `self.ReceiveBeginPlay`
  (`self.RunBehaviorTree` "/Game/Enemies/SKnight/BT_SKnightEnemy.BT_SKnightEnemy"))

(event `self.AIPerception.OnTargetPerceptionUpdated`
  (params (Actor :type "Actor Object Reference") (Stimulus :type "AIStimulus Structure"))
  (`self.HandleSightSense` Actor Stimulus))

(fn `HandleSightSense`
  (params (Actor :type "Actor Object Reference") (Stimulus :type "AIStimulus Structure"))
  (bind _returnvalue (`GameplayStatics.GetPlayerCharacter` 0))
  (bind (_stimulus_age _stimulus_expirationage _stimulus_strength _stimulus_stimuluslocation _stimulus_receiverlocation _stimulus_tag _stimulus_bsuccessfullysensed) (break `AIStimulus` (`local.Stimulus`)))
  (bind _returnvalue_2 (`AIPerceptionSystem.GetSenseClassForStimulus` Stimulus))
  (if (== _returnvalue_2 "/Script/AIModule.AISense_Sight")
    (if (== (`local.Actor`) _returnvalue)
      (`BlackboardComponent.SetValueAsObject` (`self.Blackboard`) "TargetActor" (`KismetMathLibrary.SelectObject` _returnvalue null _stimulus_bsuccessfullysensed))
      (if (not _stimulus_bsuccessfullysensed)
        (`BlackboardComponent.SetValueAsVector` (`self.Blackboard`) "LastKnownLocation" _stimulus_stimuluslocation))
      (else
        (return)))
    (else
      (return))))

(fn `UserConstructionScript`)